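; ALSX equip item component that marks which item in a named inventory on the same actor is active.
; On Tick it finds the owner's ALSX_InventoryComponent by object name and caches it, retrying until found.
; When ActiveIndex differs from LastIndex, it clears IsActive on the previous item and sets it on the new one, ignoring out-of-range indices.
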(event EventTick
  (params (DeltaSeconds :type Float%20%28single-precision%29))
  (bind _activeindex (Variables|Default|GetActiveIndex))
  (Utilities|IsValid (Variables|Default|GetInventory)
    (:Is%20Valid
      (if (not (== (Variables|Private|GetLastIndex) (Variables|Default|GetActiveIndex))) :!label _label
        (CallFunction|SetItemActive (Variables|Private|GetLastIndex) false)
        (Variables|Private|SetLastIndex _activeindex)
        (CallFunction|SetItemActive _activeindex true)))
    (:Is%20Not%20Valid
      (bind (_success _inventory) (CallFunction|FindInventory))
      (if _success
        (Variables|Default|SetInventory _inventory)
        (goto _label)))))

(fn FindInventory
  (for _array_element (Actor|GetComponentsByClass (Components|GetOwner) "/Game/ALSX/Blueprints/Inventory/ALSX_InventoryComponent.ALSX_InventoryComponent_C")
    (if (Utilities|Enum|Equal(Enum) (Utilities|GetObjectName _array_element) (Variables|Default|GetInventoryName))
      (return true _array_element)))
  (return false 0))

(fn SetItemActive
  (params (Index :type Integer) (IsEquipped :type Boolean))
  (bind _inventory (Variables|Default|GetInventory))
  (bind _items (Variables|/Game/ALSX/Blueprints/Inventory/ALSX_InventoryComponent.ALSX_InventoryComponent_C|GetItems _inventory))
  (Utilities|IsValid _inventory
    (:Is%20Valid
      (if (and (< Index (Utilities|Array|Length _items)) (>= Index 0))
        (Variables|/Game/ALSX/Blueprints/Inventory/ALSX_InventoryItem.ALSX_InventoryItem_C|SetIsActive (Utilities|Array|Get(acopy) _items Index) IsEquipped)))))