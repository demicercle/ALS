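; Actor component for a fixed-size item inventory with one equipped slot, which creates an inventory widget for the owning player on BeginPlay.
; AddItem spawns the item actor into the first empty slot, attaches it to a socket on the owner and initializes it from item data.
; CycleItem moves the active index with wraparound, and Tick detects the change, swaps Equip and Unequip, then fires the OnChanged dispatcher.
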(event Custom|OnChanged_Event_0)

(event EventTick
  (params (DeltaSeconds :type Float%20%28single-precision%29))
  (bind _activeindex (Variables|Default|GetActiveIndex))
  (if (not (== (Variables|Private|GetLastIndex) _activeindex))
    (CallFunction|SetItemEquipped (Variables|Private|GetLastIndex) false)
    (bind _output_get (Variables|Private|SetLastIndex _activeindex))
    (CallFunction|SetItemEquipped _output_get true)
    (Default|CallOnChanged)))

(event EventBeginPlay
  (bind _items (Variables|Default|GetItems))
  (EventDispatchers|AssignOnChanged (delegate Custom|OnChanged_Event_0))
  (while (< (Utilities|Array|Length _items) (Variables|Default|GetSize))
    (Utilities|Array|Add _items 0))
  (bind _aspawn (Utilities|Casting|CastToPawn (Components|GetOwner)))
  (bind _asplayer_controller (Utilities|Casting|CastToPlayerController (Pawn|GetController _aspawn)))
  (bind _returnvalue (UserInterface|CreateWidget (Variables|Default|GetWidgetClass) _asplayer_controller))
  (UserInterface|Viewport|AddtoViewport _returnvalue 0)
  (bind _asalsx_inventory_widget (Utilities|Casting|CastToALSX_InventoryWidget _returnvalue))
  (Variables|/Game/ALSX/Widgets/ALSX_InventoryWidget.ALSX_InventoryWidget_C|SetInventory _asalsx_inventory_widget self))

(fn AddItem
  (params (ItemData :type ALSX%20Item%20Data%20Object%20Reference))
  (bind _returnvalue (Components|GetOwner))
  (bind _items (Variables|Default|GetItems))
  (for (_array_element _array_index) _items
    (Utilities|IsValid _array_element
      (:Is%20Not%20Valid
        (bind _returnvalue_2 (Game|SpawnActorfromClass (Variables|/Game/ALSX/Blueprints/Inventory/ALSX_ItemData.ALSX_ItemData_C|GetActorClass ItemData) (Transformation|GetActorTransform _returnvalue) "AlwaysSpawn" _returnvalue (.AsPawn (Utilities|Casting|CastToPawn _returnvalue))))
        (Transformation|AttachActorToActor _returnvalue_2 _returnvalue (Variables|Default|GetSocketName) "SnapToTarget" "SnapToTarget" "SnapToTarget" true)
        (Utilities|Array|SetArrayElem _items _array_index _returnvalue_2)
        (Default|Init _returnvalue_2 ItemData)
        (CallFunction|SetItemEquipped _array_index (== _array_index (Variables|Default|GetActiveIndex)))
        (Default|CallOnChanged)
        (return true _returnvalue_2))))
  (return false 0))

(fn SetItemEquipped
  (params (Index :type Integer) (IsEquipped :type Boolean))
  (bind _items (Variables|Default|GetItems))
  (bind _output (Utilities|Array|Get(acopy) _items Index))
  (Utilities|IsValid _output
    (:Is%20Valid
      (if (Math|Boolean|ANDBoolean (< Index (Utilities|Array|Length _items)) (>= Index 0) (Utilities|IsValid _output))
        (bind _output_get (Variables|/Game/ALSX/Blueprints/Inventory/ALSX_InventoryItem.ALSX_InventoryItem_C|SetIsActive _output IsEquipped))
        (if _output_get
          (Default|Equip _output)
          (else
            (Default|Unequip _output)))))))

(fn CycleItem
  (params (Delta :type Integer))
  (bind _returnvalue (Math|Integer|Absolute(Integer) Delta))
  (bind _size (Variables|Default|GetSize))
  (if (>= _returnvalue 1)
    (for _index (range 1 _returnvalue)
      (if (< Delta 0)
        (Math|Integer|DecrementInt (Variables|Default|GetActiveIndex)
          (:%20%20
            (if (< (Variables|Default|GetActiveIndex) 0)
              (Variables|Default|SetActiveIndex (- _size 1)))))
        (else
          (Math|Integer|IncrementInt (Variables|Default|GetActiveIndex)
            (:%20%20
              (if (>= (Variables|Default|GetActiveIndex) _size)
                (Variables|Default|SetActiveIndex 0)))))))))

(fn GetEquippedItem
  (bind _items (Variables|Default|GetItems))
  (bind _activeindex (Variables|Default|GetActiveIndex))
  (bind _output (Utilities|Array|Get(acopy) _items _activeindex))
  (if (and (>= _activeindex 0) (< _activeindex (Utilities|Array|Length _items)))
    (Utilities|IsValid _output
      (:Is%20Valid
        (return _output)))))