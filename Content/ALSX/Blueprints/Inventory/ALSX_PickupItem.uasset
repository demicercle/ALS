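; World pickup actor that gives its ItemData to an overlapping actor's ALSX_InventoryComponent, destroying itself when the add succeeds.
; The construction script applies the item's static and skeletal meshes, hiding both without valid data.
; ResizeComponent optionally scales and centers meshes to the Sphere using their bounds (AutoSize, AutoCenter).
; After a short BeginPlay delay, it reapplies the static mesh or destroys itself if ItemData is invalid.
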(event EventBeginPlay
  (bind _itemdata (Variables|Default|GetItemData))
  (Utilities|FlowControl|Delay 0.2)
  (Utilities|IsValid _itemdata
    (:Is%20Valid
      (Components|StaticMesh|SetStaticMesh (Variables|Default|GetStaticMesh) (Variables|/Game/ALSX/Blueprints/Inventory/ALSX_ItemData.ALSX_ItemData_C|GetPickupMesh _itemdata)))
    (:Is%20Not%20Valid
      (Actor|DestroyActor))))

(event Collision|EventActorBeginOverlap
  (params (OtherActor :type Actor%20Object%20Reference))
  (bind _returnvalue (Actor|GetComponentbyClass OtherActor "/Game/ALSX/Blueprints/Inventory/ALSX_InventoryComponent.ALSX_InventoryComponent_C"))
  (Utilities|IsValid _returnvalue
    (:Is%20Valid
      (bind _success (Default|AddItem _returnvalue (Variables|Default|GetItemData)))
      (if _success
        (Actor|DestroyActor)))))

(fn ConstructionScript
  (CallFunction|UpdateMesh))

(fn UpdateMesh
  (bind _itemdata (Variables|Default|GetItemData))
  (bind _staticmesh (Variables|Default|GetStaticMesh))
  (bind _skeletalmesh (Variables|Default|GetSkeletalMesh))
  (bind _returnvalue (Utilities|IsValid _itemdata))
  (bind _skeletalmesh_2 (Variables|/Game/ALSX/Blueprints/Inventory/ALSX_ItemData.ALSX_ItemData_C|GetSkeletalMesh _itemdata))
  (bind _pickupmesh (Variables|/Game/ALSX/Blueprints/Inventory/ALSX_ItemData.ALSX_ItemData_C|GetPickupMesh _itemdata))
  (Rendering|SetVisibility (Variables|Default|GetSkeletalMesh) _returnvalue false)
  (if _returnvalue
    (Utilities|FlowControl|Sequence
      (:then_0
        (Components|StaticMesh|SetStaticMesh _staticmesh _pickupmesh)
        (Utilities|IsValid _pickupmesh
          (:Is%20Valid
            (CallFunction|ResizeComponent _staticmesh (StaticMesh|GetBounds _pickupmesh)))))
      (:then_1
        (Class|SkinnedMeshComponent|SetSkeletalMesh _skeletalmesh _skeletalmesh_2 true)
        (Utilities|IsValid _skeletalmesh_2
          (:Is%20Valid
            (CallFunction|ResizeComponent _skeletalmesh (StaticMesh|GetBounds _skeletalmesh_2))))))))

(fn ResizeComponent
  (params (Component :type Scene%20Component%20Object%20Reference) (Bounds :type Box%20Sphere%20Bounds%20Structure))
  (bind (_origin _boxextent _sphereradius) (Math|BoxSphereBounds|BreakBoxSphereBounds Bounds))
  (bind _sphere (Variables|Default|GetSphere))
  (bind _staticmesh (Variables|Default|GetStaticMesh))
  (bind (_origin_2 _boxextent_2 _sphereradius_2) (Collision|GetComponentBounds _sphere))
  (Transformation|SetRelativeScale3D _staticmesh (Math|Vector|SelectVector (Math|Conversions|ToVector(Float) (/ _sphereradius_2 _sphereradius)) "1.000000,1.000000,1.000000" (Variables|Default|GetAutoSize)))
  (Transformation|SetRelativeLocationAndRotation _staticmesh (Math|Vector|SelectVector (- _origin_2 (Math|Transform|TransformLocation (Transformation|GetActorTransform) _origin)) "0, 0, 0" (Variables|Default|GetAutoCenter)) "0, 0, 0" false false))