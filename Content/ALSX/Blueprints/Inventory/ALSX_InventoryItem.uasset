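; ALSX inventory item Blueprint that stores an item's data and its equipped state.
; Init stores the passed ItemData, and Equip and Unequip toggle the IsEquipped flag.
; UpdateHeldObject casts the given actor to the ALSX AnimMan character and calls AttachToHand with the item's meshes, anim class, hand side and offset.
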(fn ConstructionScript)

(fn Init
  (params (ItemData :type ALSX%20Item%20Data%20Object%20Reference))
  (Variables|Default|SetItemData ItemData))

(fn Equip
  (Variables|Default|SetIsEquipped true))

(fn Unequip
  (Variables|Default|SetIsEquipped false))

(fn UpdateHeldObject
  (params (Actor :type Actor%20Object%20Reference))
  (bind _itemdata (Variables|Default|GetItemData))
  (bind _asalsx_anim_man_character_bp (Utilities|Casting|CastToALSX_AnimMan_CharacterBP Actor))
  (Default|AttachtoHand _asalsx_anim_man_character_bp (Variables|/Game/ALSX/Blueprints/Inventory/ALSX_ItemData.ALSX_ItemData_C|GetStaticMesh _itemdata) (Variables|/Game/ALSX/Blueprints/Inventory/ALSX_ItemData.ALSX_ItemData_C|GetSkeletalMesh _itemdata) (Variables|/Game/ALSX/Blueprints/Inventory/ALSX_ItemData.ALSX_ItemData_C|GetAnimClass _itemdata) (Variables|/Game/ALSX/Blueprints/Inventory/ALSX_ItemData.ALSX_ItemData_C|GetLeftHand _itemdata) (Variables|/Game/ALSX/Blueprints/Inventory/ALSX_ItemData.ALSX_ItemData_C|GetHandOffset _itemdata))
  (return))